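; BP_Pickup is a pickup actor that shows an inspection widget with its name, type and description while held.
; It creates WBP_InspectInformation on BeginPlay, then re-adds it and rewrites its text every Tick while Holding is true.
; Pressing V while holding removes the widget.
; When not holding, removal runs only if the widget is already out of the viewport, so it does not hide a visible one.
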(event `self.ReceiveBeginPlay`
  (bind _returnvalue (`|CreateWidget` "/Game/Widgets/WBP_InspectInformation.WBP_InspectInformation_C")))

(event `self.ReceiveTick`
  (params (DeltaSeconds :type "Float (single-precision)"))
  (if (`self.bHolding`)
    (`UserWidget.AddToViewport` (stale `self.ReceiveBeginPlay` _returnvalue) 0)
    (bind _output_get (set `/Game/Widgets/WBP_InspectInformation.ObjectName` (`self.ObjectName`) (stale `self.ReceiveBeginPlay` _returnvalue)))
    (`TextBlock.SetText` (`/Game/Widgets/WBP_InspectInformation.Object_Name` (stale `self.ReceiveBeginPlay` _returnvalue)) _output_get)
    (bind _output_get_2 (set `self.ObjectType` (`self.ObjectType`)))
    (`TextBlock.SetText` (`/Game/Widgets/WBP_InspectInformation.Object_Type` (stale `self.ReceiveBeginPlay` _returnvalue)) _output_get_2)
    (bind _output_get_3 (set `self.ObjectDescription` (`self.ObjectDescription`)))
    (`TextBlock.SetText` (`/Game/Widgets/WBP_InspectInformation.Object_Description` (stale `self.ReceiveBeginPlay` _returnvalue)) _output_get_3)
    (if (`PlayerController.WasInputKeyJustPressed` (`GameplayStatics.GetPlayerController` 0) "V")
      (`Widget.RemoveFromParent` (stale `self.ReceiveBeginPlay` _returnvalue)))
    (elif (not (`Widget.IsInViewport` (stale `self.ReceiveBeginPlay` _returnvalue)))
      (`Widget.RemoveFromParent` (stale `self.ReceiveBeginPlay` _returnvalue)))))

(fn `UserConstructionScript`)